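; BP_Guid_GameMode is a game mode Blueprint that initializes and restarts the game session state.
; BeginPlay and the RestartGame event both call StartGame, which resets level, score, statue count, time and the game-over flag.
; StartGame then sets a one-second timer on a function named Clock, which is not defined in this file.
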(event Custom|RestartGame
  (Utilities|StartGame))

(event EventBeginPlay
  (Utilities|StartGame))

(fn ConstructionScript)